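; BP_GlobalCoin is a coin pickup that adds to the player's coin count.
; Its sphere's begin overlap runs a two-step sequence, matching the other actor against player 0's BP_MainPlayerCharacter or casting it to BP_MainPlayerCharacter2, with both paths sharing one check.
; On a match, SpawnCoin, despite its name, destroys the coin and adds 100 to Coincnt in GlobalGameInstance.
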(event OnComponentBeginOverlap(Sphere)
  (params (OverlappedComponent :type Primitive%20Component%20Object%20Reference) (OtherActor :type Actor%20Object%20Reference) (OtherComp :type Primitive%20Component%20Object%20Reference) (OtherBodyIndex :type Integer) (bFromSweep :type Boolean) (SweepResult :type Hit%20Result%20Structure%20%28by%20ref%29))
  (Variables|Default|SetOther%20Actor OtherActor)
  (Utilities|FlowControl|Sequence
    (:then_0
      (bind _asbp_main_player_character (Utilities|Casting|CastToBP_MainPlayerCharacter (Game|GetPlayerCharacter 0))))
    (:then_1
      (bind _asbp_main_player_character_2 (Utilities|Casting|CastToBP_MainPlayerCharacter2 OtherActor))))
  (if (or (== (Variables|Default|GetOther%20Actor) _asbp_main_player_character) (== _asbp_main_player_character_2 (Variables|Default|GetOther%20Actor)))
    (CallFunction|SpawnCoin)))

(event EventBeginPlay)

(event Collision|EventActorBeginOverlap
  (params (OtherActor :type Actor%20Object%20Reference)))

(event EventTick
  (params (DeltaSeconds :type Float%20%28single-precision%29)))

(fn ConstructionScript)

(fn SpawnCoin
  (Actor|DestroyActor)
  (bind _asglobal_game_instance (Utilities|Casting|CastToGlobalGameInstance (Game|GetGameInstance)))
  (Variables|/Script/RPG_Project.GlobalGameInstance|SetCoincnt _asglobal_game_instance (+ (Variables|/Script/RPG_Project.GlobalGameInstance|GetCoincnt _asglobal_game_instance) 100)))