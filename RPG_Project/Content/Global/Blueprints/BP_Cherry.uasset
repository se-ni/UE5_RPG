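; BP_Cherry is a cherry pickup item with a look-at prompt and a coin reward.
; LookAt reads the item's data table row through ItemDataComponent and returns a "Pickup {item}" label.
; AddCoin adds a fixed amount to the coin count on BP_GlobalGameInstance, though nothing in this file calls it.
; Destruction plays a 2D coin sound, while the Interactwith event is empty here.
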(event EventBeginPlay)

(event Collision|EventActorBeginOverlap
  (params (OtherActor :type Actor%20Object%20Reference)))

(event EventDestroyed
  (Audio|PlaySound2D "/Game/Sound/Coin_5.Coin_5" 1.0 1.0 0.0 0 0))

(event EventInteractwith
  (params (Stage3_PlayerCharacter :type BP%20Main%20Player%20Character%203%20Object%20Reference)))

(fn ConstructionScript)

(fn AddCoin
  (bind _asbp_global_game_instance (Utilities|Casting|CastToBP_GlobalGameInstance (Game|GetGameInstance)))
  (Variables|/Script/RPG_Project.GlobalGameInstance|SetCoincnt _asbp_global_game_instance (+ (Variables|/Script/RPG_Project.GlobalGameInstance|GetCoincnt _asbp_global_game_instance) 100)))

(fn Lookat
  (bind _itemdatacomponent (Variables|Default|GetItemDataComponent))
  (bind _itemid (Variables|/Game/Inventory/ItemDataComponent.ItemDataComponent_C|GetItemID _itemdatacomponent))
  (bind _returnvalue (Utilities|GetDataTableRow (.datatable _itemid) (.rowname _itemid))
    (:then
      (return (Utilities|Text|FormatText "Pickup {item}" (.Name (Utilities|Struct|BreakFItemStruct _returnvalue)))))))