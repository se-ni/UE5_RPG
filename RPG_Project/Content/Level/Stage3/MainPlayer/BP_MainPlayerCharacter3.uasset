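; Stage 3 player character, handling weapon attack power and the player's inventory, shop and portal inputs.
; BeginPlay hides Terrain-tagged actors from its scene capture and creates a hidden monster info widget.
; Tick compares the weapon mesh against three WeaponArrays entries to set base, pre-buff attack (LocalATT).
; Inputs open an inventory widget, show the HUD shop when OpenShop is set, and load Stage3_Level2 when OpenLevel is set.
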(event EventBeginPlay
  (Variables|Default|SetmainPlayer self)
  (bind _outactors (Actor|GetAllActorswithTag "Terrain"))
  (Variables|/Script/Engine.SceneCaptureComponent|SetHiddenActors (Variables|Default|GetSceneCaptureComponent2D) _outactors)
  (bind _returnvalue (UserInterface|CreateWidget "/Game/Level/Stage3/UI/WBP_MonsterInfo3.WBP_MonsterInfo3_C"))
  (bind _output_get (Variables|Default|SetMonsterInfo3 _returnvalue))
  (UserInterface|Viewport|AddtoViewport _output_get 0)
  (Widget|SetVisibility _output_get "Hidden"))

(event EventTick
  (params (DeltaSeconds :type Float%20%28single-precision%29))
  (bind _self self)
  (Utilities|FlowControl|Sequence
    (:then_0
      ;[1 1 1] 무기별 기본 공격력(버프 전)
      (bind _ismesh0 (CallFunction|GetStaticMesh0 _self))
      (if _ismesh0
        (Variables|Default|SetLocalATT 0.3)))
    (:then_1
      (bind _ismesh1 (CallFunction|GetStaticMesh1 _self))
      (if _ismesh1
        (Variables|Default|SetLocalATT 0.5)))
    (:then_2
      (bind _ismesh2 (CallFunction|GetStaticMesh2 _self))
      (if _ismesh2
        (Variables|Default|SetLocalATT 0.7)))))

(event Input|ActionEvents|InputActionPortal
  (params (Key :type Key%20Structure))
  (:Pressed
    (if (Variables|Default|GetOpen%20Level)
      (Game|OpenLevel(byObjectReference) "/Game/Level/Stage3_Level2.Stage3_Level2"))))

(event Input|ActionEvents|InputActionInven
  (params (Key :type Key%20Structure))
  (:Pressed
    (bind _returnvalue (UserInterface|CreateWidget "/Game/Inventory/UI/WBP_InvenWidget.WBP_InvenWidget_C"))
    (UserInterface|Viewport|AddtoViewport _returnvalue 0)))

(event Input|ActionEvents|InputActionShop
  (params (Key :type Key%20Structure))
  (:Pressed
    (if (Variables|Default|GetOpen%20Shop)
      (Widget|RemovefromParent (Variables|Default|GetUIO))
      (bind _mainwidget (CallFunction|GetMainWidget))
      (Variables|/Script/RPG_Project.MainWidget|SetShopUIOnOff _mainwidget "Visible"))))

(fn ConstructionScript)

(fn GetMainWidget
  (bind _asmain_hud (Utilities|Casting|CastToMainHUD (HUD|GetHUD (Game|GetPlayerController 0))))
  (return (Variables|/Script/RPG_Project.MainHUD|GetUIMainWidget _asmain_hud)))

(fn GetStaticMesh0
  (return (== (Variables|/Script/Engine.StaticMeshComponent|GetStaticMesh (Variables|/Script/RPG_Project.MainPlayerCharacter|GetWeaponMesh (Variables|Default|GetmainPlayer))) (Utilities|Array|Get(acopy) (Variables|/Script/RPG_Project.MainPlayerCharacter|GetWeaponArrays (Variables|Default|GetmainPlayer))))))

(fn GetStaticMesh1
  (return (== (Variables|/Script/Engine.StaticMeshComponent|GetStaticMesh (Variables|/Script/RPG_Project.MainPlayerCharacter|GetWeaponMesh (Variables|Default|GetmainPlayer))) (Utilities|Array|Get(acopy) (Variables|/Script/RPG_Project.MainPlayerCharacter|GetWeaponArrays (Variables|Default|GetmainPlayer)) 1))))

(fn GetStaticMesh2
  (return (== (Variables|/Script/Engine.StaticMeshComponent|GetStaticMesh (Variables|/Script/RPG_Project.MainPlayerCharacter|GetWeaponMesh (Variables|Default|GetmainPlayer))) (Utilities|Array|Get(acopy) (Variables|/Script/RPG_Project.MainPlayerCharacter|GetWeaponArrays (Variables|Default|GetmainPlayer)) 2))))