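; BP_StatusPlayer4 is a Stage 3 player Blueprint that handles status capture, level travel and inventory input.
; On BeginPlay it limits its SceneCapture2D show-only list to actors tagged "Status".
; The Portal input opens Stage3_Level2 when the OpenLevel flag is true; this graph never sets that flag.
; Each Inven press creates a new inventory widget on the viewport, and the removal node is unconnected.
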(event EventBeginPlay
  (bind _outactors (Actor|GetAllActorswithTag "Status"))
  (Variables|/Script/Engine.SceneCaptureComponent|SetShowOnlyActors (Variables|Default|GetStatusCaptureComponent2D) _outactors))

(event Collision|EventActorBeginOverlap
  (params (OtherActor :type Actor%20Object%20Reference)))

(event EventTick
  (params (DeltaSeconds :type Float%20%28single-precision%29)))

(event Input|ActionEvents|InputActionPortal
  (params (Key :type Key%20Structure :default "None"))
  (:Pressed
    (if (Variables|Default|GetOpen%20Level)
      (Game|OpenLevel(byObjectReference) "/Game/Level/Stage3/Stage3_Level2.Stage3_Level2"))))

(event Input|ActionEvents|InputActionInven
  (params (Key :type Key%20Structure :default "None"))
  (:Pressed
    (bind _returnvalue (UserInterface|CreateWidget "/Game/Inventory/UI/WBP_InvenWidget.WBP_InvenWidget_C"))
    (UserInterface|Viewport|AddtoViewport _returnvalue 0)))

(fn ConstructionScript)