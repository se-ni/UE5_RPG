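; BP_Portal3 is a Stage 3 portal that lets the player open a level once the monster kill count is met.
; Any overlap adds a WBP_UIP widget to the viewport, and the Capsule's end overlap removes it.
; For the player, overlap sets OpenLevel on the character if GlobalGameInstance's DeathMonster2 equals Monster2Cnt, and leaving clears it.
; The level load itself happens outside this Blueprint.
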(event OnComponentEndOverlap(Capsule)
  (params (OverlappedComponent :type Primitive%20Component%20Object%20Reference) (OtherActor :type Actor%20Object%20Reference) (OtherComp :type Primitive%20Component%20Object%20Reference) (OtherBodyIndex :type Integer))
  (Widget|RemovefromParent (Variables|Default|GetUI_P))
  (bind _asbp_main_player_character_2 (Utilities|Casting|CastToBP_MainPlayerCharacter2 (Game|GetPlayerCharacter 0)))
  (if (== (Variables|Default|GetOther%20Actor) _asbp_main_player_character_2)
    (Variables|/Game/Level/Stage2/MainPlayer/BP_MainPlayerCharacter2.BP_MainPlayerCharacter2_C|SetOpenLevel _asbp_main_player_character_2 false)))

(event Collision|EventActorBeginOverlap
  (params (OtherActor :type Actor%20Object%20Reference))
  (Variables|Default|SetOther%20Actor OtherActor)
  (CallFunction|CreateWidgetUI)
  (bind _asbp_main_player_character_2 (Utilities|Casting|CastToBP_MainPlayerCharacter2 (Game|GetPlayerCharacter 0)))
  (if (== _asbp_main_player_character_2 (Variables|Default|GetOther%20Actor))
    (bind _asglobal_game_instance (Utilities|Casting|CastToGlobalGameInstance (Game|GetGameInstance)))
    (if (== (Variables|/Script/RPG_Project.GlobalGameInstance|GetDeathMonster2 _asglobal_game_instance) (Variables|/Script/RPG_Project.GlobalGameInstance|GetMonster2Cnt _asglobal_game_instance))
      (Variables|/Game/Level/Stage2/MainPlayer/BP_MainPlayerCharacter2.BP_MainPlayerCharacter2_C|SetOpenLevel _asbp_main_player_character_2 true)
      (Development|PrintString (Utilities|String|ToString(Boolean) false)))))

(fn ConstructionScript)

(fn CreateWidgetUI
  (bind _returnvalue (UserInterface|CreateWidget "/Game/Level/Stage1/UI/WBP_UIP.WBP_UIP_C"))
  (UserInterface|Viewport|AddtoViewport _returnvalue 0)
  (Variables|Default|SetUI_P _returnvalue))

(fn CreateUIWidget)