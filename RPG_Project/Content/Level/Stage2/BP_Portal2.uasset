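; BP_Portal2 is a Stage 2 portal that detects when the player may advance to the next level.
; On capsule overlap by the BP_MainPlayerCharacter2 player, it compares Monster2Cnt with DeathMonster2 in GlobalGameInstance.
; When the counts match it only prints a "Next Level" message.
; An Open Level node targeting Stage1_Level is left unconnected, so no level change happens.
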(event OnComponentBeginOverlap(Capsule)
  (params (OverlappedComponent :type Primitive%20Component%20Object%20Reference) (OtherActor :type Actor%20Object%20Reference) (OtherComp :type Primitive%20Component%20Object%20Reference) (OtherBodyIndex :type Integer) (bFromSweep :type Boolean) (SweepResult :type Hit%20Result%20Structure%20%28by%20ref%29))
  (bind _asbp_main_player_character_2 (Utilities|Casting|CastToBP_MainPlayerCharacter2 (Game|GetPlayerCharacter 0)))
  (if (== OtherActor _asbp_main_player_character_2)
    (bind _asglobal_game_instance (Utilities|Casting|CastToGlobalGameInstance (Game|GetGameInstance)))
    (if (== (Variables|/Script/RPG_Project.GlobalGameInstance|GetMonster2Cnt _asglobal_game_instance) (Variables|/Script/RPG_Project.GlobalGameInstance|GetDeathMonster2 _asglobal_game_instance))
      (Development|PrintString "Next Level"))))

(event EventBeginPlay)

(event Collision|EventActorBeginOverlap
  (params (OtherActor :type Actor%20Object%20Reference)))

(event EventTick
  (params (DeltaSeconds :type Float%20%28single-precision%29)))

(fn ConstructionScript)