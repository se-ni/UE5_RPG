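; Brown boomerang projectile actor that flies along its facing direction, with no return-flight logic in its graphs.
; On BeginPlay it sets the ProjectileMovement velocity from its forward vector at an effectively fixed speed.
; When the projectile stops, it damages the hit actor and spawns a Niagara impact effect aligned to the surface normal.
; It then deactivates its boomerang effect, disables sphere collision and destroys itself after a short delay.
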(event OnProjectileStop(ProjectileMovement)
  (params (ImpactResult :type Hit%20Result%20Structure%20%28by%20ref%29))
  (bind (_bblockinghit _binitialoverlap _time _distance _location _impactpoint _normal _impactnormal _physmat _hitactor) (Collision|BreakHitResult ImpactResult))
  (Variables|Default|SetImpact%20Result ImpactResult)
  (Game|Damage|ApplyDamage _hitactor 5.0 0 self)
  (Niagara|SpawnSystematLocation "/Game/Assorted_Projectiles/Particles/Boomerang/Brown/NS_Boomerang_Impact_Brown.NS_Boomerang_Impact_Brown" _impactpoint (Math|Rotator|CombineRotators (Math|Conversions|RotationFromXVector _impactnormal) "0, 0, 0"))
  (Components|Activation|SetActive (Variables|Default|GetNS_Boomerang) false false)
  (Collision|SetCollisionEnabled (Variables|Default|GetSphere) "NoCollision")
  (Utilities|FlowControl|Delay 3.0)
  (Actor|DestroyActor))

(event EventBeginPlay
  (Variables|/Script/Engine.MovementComponent|SetVelocity (Variables|Default|GetProjectileMovement) (* (Math|Vector|GetForwardVector (Transformation|GetActorRotation)) (Math|Random|RandomFloatinRange 1.5e+03 1.5e+03))))

(fn ConstructionScript)