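; BP_Spawner02 is a spawner actor that repeatedly fires a configurable projectile class.
; On BeginPlay, if the class is valid, it starts a looping timer with a configurable interval and spawns once immediately.
; Each spawn places the projectile at the actor's location with the Arrow component's world rotation, ignoring collisions.
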(event Custom|Spawn
  (Game|SpawnActorfromClass (Variables|Default|GetProjectile) (Math|Transform|MakeTransform (Transformation|GetActorLocation) (Transformation|GetWorldRotation (Variables|Default|GetArrow))) "AlwaysSpawn" 0 0))

(event EventBeginPlay
  (if (Utilities|IsValidClass (Variables|Default|GetProjectile))
    (Utilities|Time|SetTimerbyEvent (delegate Custom|Spawn) (Variables|Default|GetTime) true)
    (CallFunction|Spawn)))

(fn ConstructionScript)