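; Item effect Blueprint that heals the player as soon as it spawns.
; On BeginPlay it runs the parent logic, casts player character 0 to BP_MainPlayerCharacter3 and adds a fixed amount to PlayerHP.
; This graph applies no maximum HP clamp and does not destroy the actor afterward.
; Overlap and Tick events are disabled placeholders.
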(event EventBeginPlay
  (|CallParentFunction)
  (bind _asbp_main_player_character_3 (Utilities|Casting|CastToBP_MainPlayerCharacter3 (Game|GetPlayerCharacter 0)))
  (Variables|/Script/RPG_Project.MainPlayerCharacter|SetPlayerHP _asbp_main_player_character_3 (+ (Variables|/Script/RPG_Project.MainPlayerCharacter|GetPlayerHP _asbp_main_player_character_3) 2e+01)))

(event Collision|EventActorBeginOverlap
  (params (OtherActor :type Actor%20Object%20Reference))
  (|CallParentFunction OtherActor) ; 지금 이 노드는 비활성 상태입니다. \n핀을 끌어서 다른 노드를 연결하면 활성화됩니다.
)

(event EventTick
  (params (DeltaSeconds :type Float%20%28single-precision%29))
  (|CallParentFunction DeltaSeconds) ; 지금 이 노드는 비활성 상태입니다. \n핀을 끌어서 다른 노드를 연결하면 활성화됩니다.
)

(fn ConstructionScript
  (|CallParentFunction))