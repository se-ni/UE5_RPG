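; Item effect actor for the Crate that gives the player character a temporary attack buff as soon as it begins play.
; BeginPlay sets ATTbuff on player 0's BP_MainPlayerCharacter3 and starts a one-shot timer of BuffTime length that clears it.
; Tick overwrites PlayerATT every frame, using a fixed value while buffed and LocalATT otherwise.
; TestFunc only prints a debug string.
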(event Custom|AttReset
  (Variables|/Script/RPG_Project.MainPlayerCharacter|SetATTbuff (Variables|Default|GetBP%20Main%20Player%20Character%203) false))

(event EventBeginPlay
  (|CallParentFunction)
  (bind _asbp_main_player_character_3 (Utilities|Casting|CastToBP_MainPlayerCharacter3 (Game|GetPlayerCharacter 0)))
  (Variables|Default|SetBP%20Main%20Player%20Character%203 _asbp_main_player_character_3)
  (Variables|/Script/RPG_Project.MainPlayerCharacter|SetATTbuff (Variables|Default|GetBP%20Main%20Player%20Character%203) true)
  (Utilities|Time|SetTimerbyEvent (delegate Custom|AttReset) (Variables|/Game/Level/Stage3/MainPlayer/BP_MainPlayerCharacter3.BP_MainPlayerCharacter3_C|GetBuffTime (Variables|Default|GetBP%20Main%20Player%20Character%203))) ; 1분동안 공격력 버프
)

(event Collision|EventActorBeginOverlap
  (params (OtherActor :type Actor%20Object%20Reference))
  (|CallParentFunction OtherActor) ; 지금 이 노드는 비활성 상태입니다. \n핀을 끌어서 다른 노드를 연결하면 활성화됩니다.
)

(event EventTick
  (params (DeltaSeconds :type Float%20%28single-precision%29))
  (bind _bp_main_player_character_3 (Variables|Default|GetBP%20Main%20Player%20Character%203))
  (|CallParentFunction DeltaSeconds)
  (if (Variables|/Script/RPG_Project.MainPlayerCharacter|GetATTbuff (Variables|Default|GetBP%20Main%20Player%20Character%203))
    (Variables|/Script/RPG_Project.MainPlayerCharacter|SetPlayerATT _bp_main_player_character_3 1.0)
    (else
      (Variables|/Script/RPG_Project.MainPlayerCharacter|SetPlayerATT _bp_main_player_character_3 (Variables|/Game/Level/Stage3/MainPlayer/BP_MainPlayerCharacter3.BP_MainPlayerCharacter3_C|GetLocalATT _bp_main_player_character_3)))))

(fn ConstructionScript
  (|CallParentFunction))

(fn TestFunc
  (Development|PrintString "Att"))